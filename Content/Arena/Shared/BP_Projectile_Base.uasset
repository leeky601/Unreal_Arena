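; Base projectile Blueprint for the Arena that handles the cosmetic sound and Niagara effects of a projectile.
; BeginPlay plays a spawn sound, attaches a flying sound to the root and spawns an effect facing the actor's forward vector.
; OnSpawnProjectileHitImpact plays the hit sound and effect at the supplied location.
; Each asset is validity-checked, so any can be left unset; movement and hit detection are not in these graphs.
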(event `self.ReceiveBeginPlay`
  (`|ExecutionSequence`
    (:`then_0`
      (bind _projectilespawnsound (`self.ProjectileSpawnSound`)
        (:`then`
          (`GameplayStatics.PlaySoundAtLocation` _projectilespawnsound (`self.K2_GetActorLocation`) (struct) 1.0 1.0 0.0 null null null null))
        (:`else`)))
    (:`then_1`
      (bind _projectileflyingsound (`self.ProjectileFlyingSound`)
        (:`then`
          (`GameplayStatics.SpawnSoundAttached` _projectileflyingsound (`self.RootComponent`) "None" (0.0 0.0 0.0) (struct) "KeepRelativeOffset" true 1.0 1.0 0.0 null null))
        (:`else`)))
    (:`then_2`
      (bind _projectilespawnfx (`self.ProjectileSpawnFX`)
        (:`then`
          (`NiagaraFunctionLibrary.SpawnSystemAtLocation` _projectilespawnfx (`self.K2_GetActorLocation`) (`KismetMathLibrary.Conv_VectorToRotator` (`self.GetActorForwardVector`))))
        (:`else`)))))

(event `self.BP_OnSpawnProjectileHitImpact`
  (params (HitLocation :type "Vector Structure (by ref)"))
  (`|ExecutionSequence`
    (:`then_0`
      (bind _projectilehitsound (`self.ProjectileHitSound`)
        (:`then`
          (`GameplayStatics.PlaySoundAtLocation` _projectilehitsound HitLocation (struct) 1.0 1.0 0.0 null null null null))
        (:`else`)))
    (:`then_1`
      (bind _projectilehitfx (`self.ProjectileHitFx`)
        (:`then`
          (`NiagaraFunctionLibrary.SpawnSystemAtLocation` _projectilehitfx HitLocation))
        (:`else`)))))

(fn `UserConstructionScript`)