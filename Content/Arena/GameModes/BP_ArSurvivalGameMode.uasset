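; Survival game mode Blueprint for the Arena that shows on-screen wave announcements as the survival state changes.
; On BeginPlay it binds to the state-changed delegate and switches on the state to show countdown or plain text widgets for incoming, current, last and completed waves.
; Reaching the final wave also overrides the spawn delay time.
; All-waves-done and player-death states only print debug strings.
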(event `self.ReceiveBeginPlay`
  (add `self.OnSurvivalGameModeStateChanged` (delegate `OnSurvivalGameModeStateChanged_Event`)))

(event `OnSurvivalGameModeStateChanged_Event` :!signature `self.OnSurvivalGameModeStateChanged`
  (params (InState :type "EArSurvivalGameModeState Enum" :default "WaitSpawnNewWaves"))
  (switch `EArSurvivalGameModeState` InState
    (:`WaitSpawnNewWaves`
      (`self.CreateWaveWidgetWithCoolDown` "New Wave Coming In" (`self.SpawnWaitingTime`)))
    (:`SpawningNewWaves`
      (`self.CreateWaveWidgetNoCount` (`|FormatText` "Wave {CurrentWaveCount}" (`self.CurrentWaveCount`)))
      (if (== (`self.CurrentWaveCount`) (`self.TotalWavesSpawn`))
        (set `self.SpawnDelayTime` 4.0)
        (`KismetSystemLibrary.Delay` 2.0)
        (`self.CreateWaveWidgetNoCount` "Last Wave")))
    (:`WaveCompleted`
      (`self.CreateWaveWidgetNoCount` (`|FormatText` "Wave {CurrentWaveCount} Completed" (`self.CurrentWaveCount`))))
    (:`AllWavesDone`
      (`KismetSystemLibrary.PrintString` "Clear" true true (struct :`G` 0.66 :`B` 1.0 :`A` 1.0) 10.0))
    (:`PlayerDied`
      (`KismetSystemLibrary.PrintString` "Died"))))

(fn `CreateWaveWidgetNoCount`
  (params (InTextToDisplay :type Text))
  (bind _returnvalue (`|CreateWidget` "/Game/Arena/Widget/GameModeWidgets/WBP_WaveNoCountDownText.WBP_WaveNoCountDownText_C"))
  (`UserWidget.AddToViewport` _returnvalue 0)
  (`TextBlock.SetText` (`/Game/Arena/Widget/GameModeWidgets/WBP_WaveNoCountDownText.TextBlock_Wave` _returnvalue) (`local.InTextToDisplay`)))

(fn `CreateWaveWidgetWithCoolDown`
  (params (InTextToDisplay :type Text) (InTotalTime :type "Float (double-precision)"))
  (bind _returnvalue (`|CreateWidget` "/Game/Arena/Widget/GameModeWidgets/WBP_WaveCountDownText.WBP_WaveCountDownText_C"))
  (`UserWidget.AddToViewport` _returnvalue 0)
  (`TextBlock.SetText` (`/Game/Arena/Widget/GameModeWidgets/WBP_WaveCountDownText.TextBlock_Wave` _returnvalue) (`local.InTextToDisplay`))
  (`/Game/Arena/Widget/GameModeWidgets/WBP_WaveCountDownText.StartCoolDown` _returnvalue (`local.InTotalTime`)))

(fn `UserConstructionScript`)